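; BP_Fishman_Customizable is a modular Fishman character whose gear pieces can be toggled on or off.
; The construction script makes the ropes, shield, skirt, spear, spikes and pouch skeletal meshes follow the nude body mesh through master pose, so they share its animation.
; A Show flag per piece sets that component's visibility, while the event graph holds no logic.
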(fn `UserConstructionScript`
  (`SkinnedMeshComponent.SetLeaderPoseComponent` (`self.SK_Ropes`) (`self.SK_Fishman_Nude_NoSpikes`) false)
  (`SkinnedMeshComponent.SetLeaderPoseComponent` (`self.SK_Shield`) (`self.SK_Fishman_Nude_NoSpikes`) false)
  (`SkinnedMeshComponent.SetLeaderPoseComponent` (`self.SK_Skirt`) (`self.SK_Fishman_Nude_NoSpikes`) false)
  (`SkinnedMeshComponent.SetLeaderPoseComponent` (`self.SK_Spear`) (`self.SK_Fishman_Nude_NoSpikes`) false)
  (`SkinnedMeshComponent.SetLeaderPoseComponent` (`self.SK_Spikes`) (`self.SK_Fishman_Nude_NoSpikes`) false)
  (`SkinnedMeshComponent.SetLeaderPoseComponent` (`self.SK_Pouch`) (`self.SK_Fishman_Nude_NoSpikes`) false)
  (`SceneComponent.SetVisibility` (`self.SK_Pouch`) (`self.ShowPouch`) false)
  (`SceneComponent.SetVisibility` (`self.SK_Ropes`) (`self.ShowRopes`) false)
  (`SceneComponent.SetVisibility` (`self.SK_Shield`) (`self.ShowShield`) false)
  (`SceneComponent.SetVisibility` (`self.SK_Skirt`) (`self.ShowSkirt`) false)
  (`SceneComponent.SetVisibility` (`self.SK_Spear`) (`self.ShowSpear`) false)
  (`SceneComponent.SetVisibility` (`self.SK_Spikes`) (`self.ShowSpikes`) false))